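; BP_PuzzleTracker counts solved puzzle sources and plays a level sequence once enough of them are solved.
; SetSource adds a solved source uniquely to an array or removes an unsolved one, printing current progress against StepCount.
; When the count first reaches StepCount, Solve latches HasBeenSolved, plays the LevelSequenceActor's sequence and prints a message; later removals do not reset it.
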(event `SetSource`
  (params (Source :type "Actor Object Reference") (Solved :type Boolean :default true))
  (if Solved
    (`KismetArrayLibrary.Array_AddUnique` (`self.StepSourceArray`) Source)
    (`self.PrintCurrentStep`)
    (if (`self.HasBeenSolved`)
      _
      (elif (>= (`KismetArrayLibrary.Array_Length` (`self.StepSourceArray`)) (`self.StepCount`))
        (`self.Solve`)))
    (else
      (bind _returnvalue (`KismetArrayLibrary.Array_RemoveItem` (`self.StepSourceArray`) Source))
      (if _returnvalue
        (`self.PrintCurrentStep`)))))

(event `Solve`
  (set `self.HasBeenSolved` true)
  (`MovieSceneSequencePlayer.Play` (`LevelSequenceActor.SequencePlayer` (`self.LevelSequenceActor`)))
  (`KismetSystemLibrary.PrintString` "Puzzle solved"))

(event `PrintCurrentStep`
  (`KismetSystemLibrary.PrintString` (`KismetStringLibrary.Concat_StrStr` "Current step: " (`KismetStringLibrary.Conv_IntToString` (`KismetArrayLibrary.Array_Length` (`self.StepSourceArray`))) "/" (`KismetStringLibrary.Conv_IntToString` (`self.StepCount`)))))

(fn `UserConstructionScript`)