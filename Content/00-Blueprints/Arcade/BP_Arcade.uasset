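; BP_Arcade is an arcade pawn that takes over player control when a controlled Character enters its Sphere, then shows a UI for its Songs.
; The overlap stores the Character and has its controller possess the arcade, provided the arcade is not already controlled.
; Possession creates BP_ArcadeWidget with the Songs, and its return button hands the controller back to the stored Character.
; Unpossession removes the widget.
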(event `self.Sphere.OnComponentBeginOverlap`
  (params (OverlappedComponent :type "PrimitiveComponent Object Reference") (OtherActor :type "Actor Object Reference") (OtherComp :type "PrimitiveComponent Object Reference") (OtherBodyIndex :type Integer) (bFromSweep :type Boolean) (SweepResult :type "HitResult Structure (by ref)"))
  (if (not (`self.IsPawnControlled`))
    (bind _ascharacter (cast `Character` OtherActor))
    (if (`self.IsPawnControlled` _ascharacter)
      (`self.Take Control from Character` _ascharacter))))

(event `Take Control from Character`
  (params (Character :type "Character Object Reference"))
  (bind _output_get (set `self.Character` Character))
  (`Controller.Possess` (`self.GetController` _output_get) self))

(event `Give Control Back to Character`
  (if (and (`self.IsControlled`) (`KismetSystemLibrary.IsValid` (`self.Character`)))
    (`Controller.Possess` (`self.GetController`) (`self.Character`))))

(event `self.ReceivePossessed`
  (params (NewController :type "Controller Object Reference"))
  (`self.Construct ArcadeWidget`))

(event `self.ReceiveUnpossessed`
  (params (OldController :type "Controller Object Reference"))
  (`self.Destroy ArcadeWidget`))

(event `Construct ArcadeWidget`
  (`self.Destroy ArcadeWidget`)
  (bind _returnvalue (`|CreateWidget` "/Game/00-Blueprints/Arcade/BP_ArcadeWidget.BP_ArcadeWidget_C" (`GameplayStatics.GetPlayerController` 0) (`self.Songs`)))
  (bind _output_get (set `self.ArcadeWidget` _returnvalue))
  (add `/Game/00-Blueprints/Arcade/BP_ArcadeWidget.OnReturnButtonClicked` _output_get (delegate `Leave Arcade`))
  (`UserWidget.AddToViewport` _output_get 0))

(event `Leave Arcade`
  (`self.Give Control Back to Character`))

(event `Destroy ArcadeWidget`
  (bind _arcadewidget (`self.ArcadeWidget`))
  (`/Engine/EditorBlueprintResources/StandardMacros.IsValid` _arcadewidget
    (:`Is Valid`
      (`Widget.RemoveFromParent` _arcadewidget)
      (set `self.ArcadeWidget` null))))

(fn `UserConstructionScript`)